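; Game state for a character customizer that supplies the items of the selected class and applies equipped items to the player's pawn.
; Selecting a class looks up its data table in a map, stores it as current, and broadcasts each row's name, type and texture through the OnItemUpdated dispatcher.
; Equipping looks up the item in that table and replaces the cached pawn's tool or helmet model according to item type.
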(event `self.ReceiveBeginPlay`
  (bind _asbp_character_pawn (cast `/Game/CharacterCustomizer/Blueprints/BP_CharacterPawn` (`GameplayStatics.GetPlayerPawn` 0)))
  (set `self.Player Pawn` _asbp_character_pawn))

(event `UpdateCharacterClass`
  (params (`Class Name` :type Name))
  (bind (_value _returnvalue) (`BlueprintMapLibrary.Map_Find` (`self.CharacterClasses`) `Class Name`))
  (if _returnvalue
    (bind _output_get (set `self.CurrentCharacterClass` _value))
    (bind _outrownames (`DataTableFunctionLibrary.GetDataTableRowNames` _output_get))
    (for _array_element _outrownames
      (bind _returnvalue_2 (`|GetDataTableRow` _output_get _array_element)
        (:`then`
          (bind (_type _damage _health _mana _model _texture) (break `/Game/CharacterCustomizer/Blueprints/Structures/S_Item` _returnvalue_2))
          (`self.OnItemUpdated` _array_element _type _texture))))))

(event `OnNewItemEquipped`
  (params (`Item Name` :type Name))
  (bind _returnvalue (`|GetDataTableRow` (`self.CurrentCharacterClass`) `Item Name`)
    (:`then`
      (bind (_type _damage _health _mana _model) (break `/Game/CharacterCustomizer/Blueprints/Structures/S_Item` _returnvalue))
      (switch `/Game/CharacterCustomizer/Blueprints/E_ItemType` _type
        (:`NewEnumerator0`
          (`/Game/CharacterCustomizer/Blueprints/BP_CharacterPawn.ReplaceTool` (`self.Player Pawn`) _model))
        (:`NewEnumerator1`
          (`/Game/CharacterCustomizer/Blueprints/BP_CharacterPawn.ReplaceHelmet` (`self.Player Pawn`) _model))))))

(fn `UserConstructionScript`)